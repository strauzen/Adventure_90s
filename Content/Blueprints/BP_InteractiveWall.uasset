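; BP_InteractiveWall is a wall that toggles between closed and open when it receives an Interact event.
; BeginPlay caches the mesh's starting relative location and derives an open location lowered along Z.
; Interact calls the Open or Close graph, which slides the mesh with a timed MoveComponentTo, easing in only when opening.
; An IsMoving flag ignores interactions mid-move, and IsOpen tracks the current state.
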(event `self.ReceiveBeginPlay`
  (bind _relativelocation (`SceneComponent.RelativeLocation` (`self.StaticMeshComponent`)))
  (set `self.OriginalLocation` _relativelocation)
  (set `self.OpenLocation` (+ _relativelocation (0.0 0.0 -400.0))))

(event `/Game/Blueprints/BPI_Interactable.Interact`
  (params (OtherActor :type "Actor Object Reference"))
  (if (not (`self.isMoving`))
    (set `self.isMoving` true)
    (if (`self.isOpen`)
      (`KismetSystemLibrary.MoveComponentTo` (`self.StaticMeshComponent`) (`self.OriginalLocation`) (struct) false false 3.0)
      (set `self.isMoving` false)
      (set `self.isOpen` false)
      (else
        (`KismetSystemLibrary.MoveComponentTo` (`self.StaticMeshComponent`) (`self.OpenLocation`) (struct) false true 3.0)
        (set `self.isMoving` false)
        (set `self.isOpen` true)))))

(fn `UserConstructionScript`)