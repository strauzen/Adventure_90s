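; BP_AdventurePawnFollowCorner turns to face a referenced Character from wherever it is placed, without moving itself.
; Each Tick it computes a look-at rotation from its own location to the Character and applies that pitch and yaw, keeping its current roll.
; The world-space result is applied as relative rotation, and the Character reference is neither assigned nor validity-checked in these graphs.
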(event `self.ReceiveTick`
  (params (DeltaSeconds :type "Float (single-precision)"))
  (`self.K2_SetActorRelativeRotation` (`KismetMathLibrary.MakeRotator` (.roll (`self.K2_GetActorRotation`)) (.pitch (`KismetMathLibrary.FindLookAtRotation` (`self.K2_GetActorLocation`) (`self.K2_GetActorLocation` (`self.Character`)))) (.yaw (`KismetMathLibrary.FindLookAtRotation` (`self.K2_GetActorLocation`) (`self.K2_GetActorLocation` (`self.Character`)))))))

(fn `UserConstructionScript`
  (`parent.UserConstructionScript`))